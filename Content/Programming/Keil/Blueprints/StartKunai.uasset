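; A spinning VR kunai pickup that starts the game by opening PearsonVRMap when grabbed.
; Pickup disables physics and snaps it to the motion controller's KunaiSocket before the level load.
; Hitting a RobotBluePrint spawns a scaled-down explosion, destroys the kunai and adds to the player controller's LimitBreak.
; The drop functions are empty stubs, and the release logic that re-enables physics and detaches is unwired.
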(event `self.ReceiveBeginPlay`
  (bind _outactors (`GameplayStatics.GetAllActorsOfClass` "/Game/Programming/Pearson/PlayerContent/PlayerController.PlayerController_C"))
  (set `self.Player` (`|GetArrayItem` _outactors)))

(event `self.ReceiveTick`
  (params (DeltaSeconds :type "Float (single-precision)"))
  (`self.K2_AddActorLocalRotation` (struct :`Yaw` 5.0 :`Roll` 10.0)))

(event `/Game/Programming/Pearson/PlayerContent/PickupActorInterface.Pickup`
  (params (AttachTo :type "SceneComponent Object Reference"))
  (set `self.Release` false)
  (`PrimitiveComponent.SetSimulatePhysics` (`self.StaticMeshComponent`) false)
  (`SceneComponent.K2_AttachToComponent` (`self.K2_GetRootComponent`) AttachTo "KunaiSocket" "SnapToTarget" "SnapToTarget" "KeepWorld" false)
  (`GameplayStatics.OpenLevel` "PearsonVRMap"))

(event `Drop_1`)

(event `self.StaticMeshComponent.OnComponentHit`
  (params (HitComponent :type "PrimitiveComponent Object Reference") (OtherActor :type "Actor Object Reference") (OtherComp :type "PrimitiveComponent Object Reference") (NormalImpulse :type "Vector Structure") (Hit :type "HitResult Structure (by ref)"))
  (bind _player (`self.Player`))
  (cast `/Game/Programming/Shawn/AI/RobotBluePrint` OtherActor)
  (bind _returnvalue (`GameplayStatics.SpawnEmitterAtLocation` "/Game/StarterContent/Particles/P_Explosion.P_Explosion" Hit_ImpactPoint (`KismetMathLibrary.Conv_VectorToRotator` Hit_ImpactNormal)))
  (`SceneComponent.SetWorldScale3D` _returnvalue (/ (`SceneComponent.K2_GetComponentScale` _returnvalue) 5.0))
  (`self.K2_DestroyActor`)
  (set `/Game/Programming/Pearson/PlayerContent/PlayerController.LimitBreak` (+ (`/Game/Programming/Pearson/PlayerContent/PlayerController.LimitBreak` _player) 10.0) _player))

(fn `Drop`
  (params (beginRelease :type "Vector Structure"))
  (returns (NewParam :type Boolean))
  (return false))

(fn `Dropp`)

(fn `UserConstructionScript`
  (bind _outactors (`GameplayStatics.GetAllActorsOfClass` "/Game/Programming/Pearson/PlayerContent/PlayerController.PlayerController_C"))
  (set `self.Player` (`|GetArrayItem` _outactors)))