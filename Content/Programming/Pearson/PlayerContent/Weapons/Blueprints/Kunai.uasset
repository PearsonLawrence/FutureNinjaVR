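; Throwable kunai weapon that a motion controller picks up and throws at enemies.
; Pickup disables physics and snaps it to the hand's KunaiSocket; Drop detaches it with a scaled impulse and throw sound.
; Once released, Tick rotates it along its velocity and destroys it after a delay.
; Hitting a robot or sentry eye deals damage, spawns a small explosion and a DamageHit actor facing the player controller, then destroys the kunai.
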(event `self.ReceiveBeginPlay`
  (bind _outactors (`GameplayStatics.GetAllActorsOfClass` "/Game/Programming/Pearson/PlayerContent/PlayerController.PlayerController_C"))
  (set `self.Player` (`|GetArrayItem` _outactors)))

(event `self.ReceiveTick`
  (params (DeltaSeconds :type "Float (single-precision)"))
  (bind _returnvalue (`KismetMathLibrary.GetForwardVector` (`self.K2_GetActorRotation`)))
  (if (`self.Release`)
    (`self.K2_SetActorRotation` (`KismetMathLibrary.FindLookAtRotation` _returnvalue (+ (`self.GetVelocity`) _returnvalue)) true)
    (`KismetSystemLibrary.Delay` 5.0)
    (`self.K2_DestroyActor`)))

(event `/Game/Programming/Pearson/PlayerContent/PickupActorInterface.Pickup`
  (params (AttachTo :type "SceneComponent Object Reference"))
  (set `self.Release` false)
  (`PrimitiveComponent.SetSimulatePhysics` (`self.StaticMeshComponent`) false)
  (`SceneComponent.K2_AttachToComponent` (`self.K2_GetRootComponent`) AttachTo "KunaiSocket" "SnapToTarget" "SnapToTarget" "KeepWorld" false))

(event `self.StaticMeshComponent.OnComponentHit`
  (params (HitComponent :type "PrimitiveComponent Object Reference") (OtherActor :type "Actor Object Reference") (OtherComp :type "PrimitiveComponent Object Reference") (NormalImpulse :type "Vector Structure") (Hit :type "HitResult Structure (by ref)"))
  (bind _asrobot_blue_print (cast `/Game/Programming/Shawn/AI/RobotBluePrint` OtherActor)
    (:`then`
      _)
    (:`CastFailed`
      (bind _assentry_eye_blue_print (cast `/Game/Programming/Shawn/AI/SentryEyeBluePrint` OtherActor))))
  (bind _returnvalue (`GameplayStatics.SpawnEmitterAtLocation` "/Game/StarterContent/Particles/P_Explosion.P_Explosion" Hit_ImpactPoint (`KismetMathLibrary.Conv_VectorToRotator` Hit_ImpactNormal)))
  (`SceneComponent.SetWorldScale3D` _returnvalue (/ (`SceneComponent.K2_GetComponentScale` _returnvalue) 5.0))
  (bind _returnvalue_2 (`|SpawnActorFromClass` "/Game/Programming/Keil/Widgets/DamageHit.DamageHit_C" (`SceneComponent.K2_GetComponentToWorld` (`self.StaticMesh`)) "Undefined" "OverrideRootScale" null null))
  (`self.K2_SetActorRotation` _returnvalue_2 (`KismetMathLibrary.Conv_VectorToRotator` (* (`KismetMathLibrary.Normal` (- (`self.K2_GetActorLocation`) (`self.K2_GetActorLocation` (`self.Player`)))) -1.0)) false)
  (set `/Game/Programming/Keil/Widgets/DamageHit.Damage` 10.0 _returnvalue_2)
  (`self.K2_DestroyActor`)
  (`/Game/Programming/Shawn/AI/RobotBluePrint.TakeDamage` _asrobot_blue_print 10.0)
  (`/Game/Programming/Shawn/AI/RobotBluePrint.TakeDamage` _assentry_eye_blue_print 10.0)
  (`KismetSystemLibrary.Delay` 0.2)
  (`self.K2_DestroyActor` _returnvalue_2))

(fn `Drop`
  (params (beginRelease :type "Vector Structure"))
  (returns (NewParam :type Boolean))
  ;[1 1 1] Add small impulse from forward of hand
  (set `self.Release` true)
  (`PrimitiveComponent.SetSimulatePhysics` (`self.StaticMeshComponent`) true)
  (`self.K2_DetachFromActor` "KeepWorld" "KeepWorld" "KeepWorld")
  (`PrimitiveComponent.AddImpulse` (`self.StaticMeshComponent`) (* beginRelease 3.0) "None" false)
  (`GameplayStatics.SpawnSoundAtLocation` "/Game/Programming/Shawn/Sounds/Ambience/kunai_throw.kunai_throw" (`SceneComponent.K2_GetComponentLocation` (`self.StaticMeshComponent`)) (struct) 0.3)
  (return false))

(fn `UserConstructionScript`
  (bind _outactors (`GameplayStatics.GetAllActorsOfClass` "/Game/Programming/Pearson/PlayerContent/PlayerController.PlayerController_C"))
  (set `self.Player` (`|GetArrayItem` _outactors)))