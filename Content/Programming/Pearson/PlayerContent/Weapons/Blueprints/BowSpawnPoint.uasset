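; BowSpawnPoint is the motion-controller grab point on the Bow that spawns arrows and sets their launch force.
; While not grabbed, it snaps to the midpoint of the first Bow found in the level every tick.
; Pickup checks player energy and the bow's release state, then attaches to the hand and spawns a linked Arrow.
; Drop sets arrow force from its distance to the bow tip, drops the arrow and detaches.
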(event `self.ReceiveBeginPlay`
  (bind _outactors (`GameplayStatics.GetAllActorsOfClass` "/Game/Programming/Pearson/PlayerContent/Weapons/Blueprints/Bow.Bow_C"))
  (set `self.bow` (`|GetArrayItem` _outactors))
  ;[1 1 1] Set location to midpoint on bow
  (`self.K2_SetActorLocation` (`SceneComponent.K2_GetComponentLocation` (`/Game/Programming/Pearson/PlayerContent/Weapons/Blueprints/Bow.MidPoint` (`self.bow`))) :!label _label))

(event `self.ReceiveTick`
  (params (DeltaSeconds :type "Float (single-precision)"))
  ;[1 1 1] Set location to midpoint on bow
  (if (not (`self.Grabbed`))
    (goto _label)))

(event `/Game/Programming/Pearson/PlayerContent/PickupActorInterface.Pickup`
  (params (AttachTo :type "SceneComponent Object Reference"))
  ;[1 1 1] Spawn Arrow on grab point
  (if (>= (`/Game/Programming/Pearson/PlayerContent/PlayerController.Energy` (`/Game/Programming/Pearson/PlayerContent/Weapons/Blueprints/Bow.Player` (`self.bow`))) 10.0)
    (if (not (`/Game/Programming/Pearson/PlayerContent/Weapons/Blueprints/Bow.Release` (`self.bow`)))
      (set `self.Grabbed` true)
      (`PrimitiveComponent.SetSimulatePhysics` (`self.Grabber`) false)
      (`SceneComponent.K2_AttachToComponent` (`self.K2_GetRootComponent`) AttachTo "KunaiSocket" "SnapToTarget" "SnapToTarget" "KeepWorld" false)
      (bind _returnvalue (`|SpawnActorFromClass` "/Game/Programming/Pearson/PlayerContent/Weapons/Blueprints/Arrow.Arrow_C" (`SceneComponent.K2_GetComponentToWorld` (`self.Grabber`)) "AlwaysSpawn" "OverrideRootScale" null null))
      (bind _output_get (set `self.Arrow` _returnvalue))
      (set `/Game/Programming/Pearson/PlayerContent/Weapons/Blueprints/Arrow.PositionOnBow` self _output_get)
      (set `/Game/Programming/Pearson/PlayerContent/Weapons/Blueprints/Arrow.Bow` (`self.bow`) _output_get))))

(fn `Drop`
  (params (beginRelease :type "Vector Structure"))
  (returns (NewParam :type Boolean))
  (bind _arrow (`self.Arrow`))
  (set `self.Grabbed` false)
  ;[1 1 1] Set Arrow Force and drop arrow
  (set `/Game/Programming/Pearson/PlayerContent/Weapons/Blueprints/Arrow.Force` (`KismetMathLibrary.VSize` (- (`self.K2_GetActorLocation`) (`SceneComponent.K2_GetComponentLocation` (`/Game/Programming/Pearson/PlayerContent/Weapons/Blueprints/Bow.Tip` (`self.bow`))))) _arrow)
  (`/Game/Programming/Pearson/PlayerContent/PickupActorInterface.Drop` _arrow (0.0 0.0 0.0))
  (`self.K2_DetachFromActor` "KeepWorld" "KeepWorld" "KeepWorld")
  (return false))

(fn `UserConstructionScript`)