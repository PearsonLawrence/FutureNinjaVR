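; VR bow weapon that the player picks up by motion controller and that returns to the player's holster when dropped.
; Pickup snaps it to the controller's KunaiSocket and hides the handle; Drop detaches it and shows the handle.
; Tick lerps the bow's scale up while held, or pins it to HolsterBow and shrinks it while released.
; Two cables attach to the first BowSpawnPoint; destruction logic exists but is unwired.
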(event `self.ReceiveBeginPlay`
  ;[1 1 1] Assaign grab points and player
  (bind _outactors (`GameplayStatics.GetAllActorsOfClass` "/Game/Programming/Pearson/PlayerContent/PlayerController.PlayerController_C"))
  (set `self.Player` (`|GetArrayItem` _outactors))
  (bind _outactors_2 (`GameplayStatics.GetAllActorsOfClass` "/Game/Programming/Pearson/PlayerContent/Weapons/Blueprints/BowSpawnPoint.BowSpawnPoint_C"))
  (bind _output_get (set `self.actor` (`|GetArrayItem` _outactors_2)))
  (`CableComponent.SetAttachEndTo` (`self.Cable2`) _output_get "None" "None")
  (`CableComponent.SetAttachEndTo` (`self.Cable`) _output_get "None" "None"))

(event `self.ReceiveTick`
  (params (DeltaSeconds :type "Float (single-precision)"))
  (bind _grow (`self.Grow`))
  (bind _grow_2 (`self.Grow`))
  (bind _relativescale3d_x (`KismetMathLibrary.BreakVector` (`SceneComponent.RelativeScale3D` _grow)))
  (bind _holster_bow (`/Game/Programming/Pearson/PlayerContent/PlayerController.Holster Bow` (`self.Player`)))
  (bind _relativescale3d_x_2 (`KismetMathLibrary.BreakVector` (`SceneComponent.RelativeScale3D` _grow_2)))
  ;[1 1 1] Grow And Shrink
  (if (`self.Release`)
    (`self.K2_SetActorLocation` (`SceneComponent.K2_GetComponentLocation` _holster_bow))
    (`self.K2_SetActorRotation` (`SceneComponent.K2_GetComponentRotation` _holster_bow))
    (if (> _relativescale3d_x_2 0.0)
      (`SceneComponent.SetRelativeScale3D` _grow_2 (`KismetMathLibrary.VLerp` (`SceneComponent.RelativeScale3D` _grow_2) (0.0 0.0 0.0) (* (`GameplayStatics.GetWorldDeltaSeconds`) 4.0))))
    (elif (< _relativescale3d_x 1.0)
      (`SceneComponent.SetRelativeScale3D` _grow (`KismetMathLibrary.VLerp` (`SceneComponent.RelativeScale3D` _grow) (1.0 1.0 1.0) (* (`GameplayStatics.GetWorldDeltaSeconds`) 6.0))))))

(event `self.Pickup`
  (params (AttachTo :type "SceneComponent Object Reference"))
  (set `self.Release` false)
  (`PrimitiveComponent.SetSimulatePhysics` (`self.StaticMeshComponent`) false)
  (`SceneComponent.K2_AttachToComponent` (`self.K2_GetRootComponent`) AttachTo "KunaiSocket" "SnapToTarget" "SnapToTarget" "KeepWorld" false)
  (`SceneComponent.SetVisibility` (`self.Handle`) false false))

(event `Drop_1`)

(fn `Drop`
  (params (beginRelease :type "Vector Structure"))
  (returns (NewParam :type Boolean))
  (if (not (`self.Destroy`))
    (set `self.Release` true)
    (`PrimitiveComponent.SetSimulatePhysics` (`self.StaticMeshComponent`) false)
    (`self.K2_DetachFromActor` "KeepWorld" "KeepWorld" "KeepWorld")
    (`SceneComponent.SetVisibility` (`self.Handle`) true false)
    (return false)))

(fn `UserConstructionScript`
  (bind _outactors (`GameplayStatics.GetAllActorsOfClass` "/Game/Programming/Pearson/PlayerContent/PlayerController.PlayerController_C"))
  (set `self.Player` (`|GetArrayItem` _outactors))
  (bind _outactors_2 (`GameplayStatics.GetAllActorsOfClass` "/Game/Programming/Pearson/PlayerContent/Weapons/Blueprints/BowSpawnPoint.BowSpawnPoint_C"))
  (bind _output_get (set `self.actor` (`|GetArrayItem` _outactors_2)))
  (`CableComponent.SetAttachEndTo` (`self.Cable2`) _output_get "None" "None")
  (`CableComponent.SetAttachEndTo` (`self.Cable`) _output_get "None" "None"))