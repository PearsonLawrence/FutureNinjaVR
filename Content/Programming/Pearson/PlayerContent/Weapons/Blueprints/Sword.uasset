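; Lightsaber-style sword actor that motion controllers pick up and use to slice procedural meshes.
; Pickup attaches it to the given component and grows the blade; Drop detaches it, after which Tick pins it to the player's katana holster and shrinks the blade.
; Blade overlaps cut MeshSlice actors along the blade's plane, add physics impulse to both halves, award player Energy and play a hit sound.
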(event `self.ReceiveBeginPlay`
  (bind _outactors (`GameplayStatics.GetAllActorsOfClass` "/Game/Programming/Pearson/PlayerContent/PlayerController.PlayerController_C"))
  (set `self.Player` (`|GetArrayItem` _outactors))
  (`GameplayStatics.SpawnSoundAttached` "/Game/Programming/Shawn/Sounds/Ambience/LightSaber.LightSaber" (`self.Grow`) "None" (0.0 0.0 0.0) (struct) "KeepRelativeOffset" false 1.0 1.0 0.0 null null false))

(event `self.ReceiveTick`
  (params (DeltaSeconds :type "Float (single-precision)"))
  (bind _grow (`self.Grow`))
  (bind _grow_2 (`self.Grow`))
  (bind _holster_katana (`/Game/Programming/Pearson/PlayerContent/PlayerController.Holster Katana` (`self.Player`)))
  (bind _relativescale3d_x (`KismetMathLibrary.BreakVector` (`SceneComponent.RelativeScale3D` _grow)))
  (bind _relativescale3d_x_2 (`KismetMathLibrary.BreakVector` (`SceneComponent.RelativeScale3D` _grow_2)))
  ;[1 1 1] Grow and shrink
  (if (`self.Release`)
    (`self.K2_SetActorLocation` (`SceneComponent.K2_GetComponentLocation` _holster_katana))
    (`self.K2_SetActorRotation` (`SceneComponent.K2_GetComponentRotation` _holster_katana))
    (if (> _relativescale3d_x 0.0)
      (`SceneComponent.SetRelativeScale3D` _grow (`KismetMathLibrary.VLerp` (`SceneComponent.RelativeScale3D` _grow) (0.0 0.0 0.0) (* (`GameplayStatics.GetWorldDeltaSeconds`) 4.0))))
    (elif (< _relativescale3d_x_2 1.0)
      (`SceneComponent.SetRelativeScale3D` _grow_2 (`KismetMathLibrary.VLerp` (`SceneComponent.RelativeScale3D` _grow_2) (1.0 1.0 1.0) (* (`GameplayStatics.GetWorldDeltaSeconds`) 6.0))))))

(event `self.Blade.OnComponentBeginOverlap`
  (params (OverlappedComponent :type "PrimitiveComponent Object Reference") (OtherActor :type "Actor Object Reference") (OtherComp :type "PrimitiveComponent Object Reference") (OtherBodyIndex :type Integer) (bFromSweep :type Boolean) (SweepResult :type "HitResult Structure (by ref)"))
  (bind _player (`self.Player`))
  (bind _blade (`self.Blade`))
  (bind _returnvalue (`SceneComponent.K2_GetComponentLocation` _blade))
  ;[1 1 1] Slice Mesh
  (bind _asmesh_slice (cast `/Game/Programming/Pearson/Misc/MeshSlice` OtherActor))
  (`/Engine/EditorBlueprintResources/StandardMacros.DoOnce` false :!label _label
    (:`Completed`
      (bind _proceduralmesh (`/Game/Programming/Pearson/Misc/MeshSlice.ProceduralMesh` _asmesh_slice))
      (bind _outotherhalfprocmesh (`KismetProceduralMeshLibrary.SliceProceduralMesh` _proceduralmesh _returnvalue (`SceneComponent.GetUpVector` _blade) true "CreateNewSectionForCap" "/Game/VirtualReality/Materials/ArrowMat.ArrowMat"))
      (`PrimitiveComponent.SetSimulatePhysics` _proceduralmesh true)
      (`PrimitiveComponent.SetSimulatePhysics` _outotherhalfprocmesh true)
      (`PrimitiveComponent.AddRadialImpulse` _outotherhalfprocmesh _returnvalue 500.0 10.0 "RIF_Constant" false)
      (`PrimitiveComponent.AddRadialImpulse` _proceduralmesh _returnvalue 500.0 10.0 "RIF_Constant" false)
      (set `/Game/Programming/Pearson/PlayerContent/PlayerController.Energy` (+ (`/Game/Programming/Pearson/PlayerContent/PlayerController.Energy` _player) 10.0) _player)
      (`GameplayStatics.SpawnSoundAtLocation` "/Game/Programming/Shawn/Sounds/Ambience/SwordHit.SwordHit" _returnvalue (struct) 0.3))))

(event `self.Blade.OnComponentEndOverlap`
  (params (OverlappedComponent :type "PrimitiveComponent Object Reference") (OtherActor :type "Actor Object Reference") (OtherComp :type "PrimitiveComponent Object Reference") (OtherBodyIndex :type Integer))
  ;[1 1 1] Slice Mesh
  (goto _label :!via `Reset`))

(event `/Game/Programming/Pearson/PlayerContent/PickupActorInterface.Pickup`
  (params (AttachTo :type "SceneComponent Object Reference"))
  (set `self.Release` false)
  (`PrimitiveComponent.SetSimulatePhysics` (`self.StaticMeshComponent`) false)
  (`SceneComponent.SetVisibility` (`self.Battery`) false false)
  (`SceneComponent.K2_AttachToComponent` (`self.K2_GetRootComponent`) AttachTo "KunaiSocket" "SnapToTarget" "SnapToTarget" "KeepWorld" false))

(fn `Drop`
  (params (beginRelease :type "Vector Structure"))
  (returns (NewParam :type Boolean))
  (set `self.Release` true)
  (`SceneComponent.SetVisibility` (`self.Battery`) true false)
  (`self.K2_DetachFromActor` "KeepWorld" "KeepWorld" "KeepWorld"))

(fn `UserConstructionScript`
  (bind _outactors (`GameplayStatics.GetAllActorsOfClass` "/Game/Programming/Pearson/PlayerContent/PlayerController.PlayerController_C"))
  (set `self.Player` (`|GetArrayItem` _outactors)))